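; BP_ButtonStartStop is a start/stop button actor whose color reflects whether the game has started.
; On BeginPlay it creates a dynamic material instance from M_buttonstartstop_Inst and applies it to its Cylinder mesh.
; Every Tick it reads the Started flag on BP_GM_MPIAGameMode and sets the colorStart parameter to red when started, green otherwise.
; It only displays state; no input or overlap logic changes that flag here.
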(event `self.ReceiveBeginPlay`
  (bind _returnvalue (`KismetMaterialLibrary.CreateDynamicMaterialInstance` "/Game/Own/buttons/M_buttonstartstop_Inst.M_buttonstartstop_Inst"))
  (bind _output_get (set `self.materialButtonStart` _returnvalue))
  (`PrimitiveComponent.SetMaterial` (`self.Cylinder`) 0 _output_get))

(event `self.ReceiveTick`
  (params (DeltaSeconds :type "Float (single-precision)"))
  (bind _asbp_gm_mpiagame_mode (cast `/Game/Own/player/BP_GM_MPIAGameMode` (`GameplayStatics.GetGameMode`)))
  (if (`MPIAGameMode.Started` _asbp_gm_mpiagame_mode)
    (`MaterialInstanceDynamic.SetVectorParameterValue` (`self.materialButtonStart`) "colorStart" (struct :`R` 1.0 :`A` 1.0))
    (else
      (`MaterialInstanceDynamic.SetVectorParameterValue` (`self.materialButtonStart`) "colorStart" (struct :`R` 0.093206 :`G` 1.0 :`A` 1.0)))))

(fn `UserConstructionScript`)
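; BP_Circuit is an actor, filed with the buttons, that visually indicates whether circuit mode is on in the game.
; Every Tick, after calling the parent Tick, it casts the game mode to BP_GM_MPIAGameMode and reads its CircuitMod flag.
; It sets the textColor parameter on the Materialins material to purple when the flag is set and white otherwise.
; The file itself only reads the flag and never changes it.
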(event `self.ReceiveTick`
  (params (DeltaSeconds :type "Float (single-precision)"))
  (`parent.ReceiveTick` DeltaSeconds)
  (bind _asbp_gm_mpiagame_mode (cast `/Game/Own/player/BP_GM_MPIAGameMode` (`GameplayStatics.GetGameMode`)))
  (if (`MPIAGameMode.CircuitMod` _asbp_gm_mpiagame_mode)
    (`MaterialInstanceDynamic.SetVectorParameterValue` (`self.materialins`) "textColor" (struct :`R` 0.423786 :`G` 0.006914 :`B` 1.0 :`A` 1.0))
    (else
      (`MaterialInstanceDynamic.SetVectorParameterValue` (`self.materialins`) "textColor" (struct :`R` 1.0 :`G` 1.0 :`B` 1.0 :`A` 1.0)))))

(fn `UserConstructionScript`
  (`parent.UserConstructionScript`))
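; BP_MainVehicule is a vehicle that steers among BP_TargetToGo actors according to the player's chosen movement mode.
; Each tick, once the MPIA game mode has started, it gathers all targets and reads ModeChoosen from the player controller.
; Mode 0 runs OneWay and mode 2 runs Circuit, while mode 1 does nothing.
; TwoWay, Arrival, Pursuit and VehiculeMovement calls sit unconnected in the graph.
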(event `self.ReceiveTick`
  (params (DeltaSeconds :type "Float (single-precision)"))
  (bind _asbp_gm_mpiagame_mode (cast `/Game/Own/player/BP_GM_MPIAGameMode` (`GameplayStatics.GetGameMode`)))
  (if (`MPIAGameMode.Started` _asbp_gm_mpiagame_mode)
    (bind _asbp_mpiaplayer_controller (cast `/Game/Own/player/BP_MPIAPlayerController` (`GameplayStatics.GetPlayerController` 0)))
    (bind _outactors (`GameplayStatics.GetAllActorsOfClass` "/Game/Own/targets/BP_TargetToGo.BP_TargetToGo_C"))
    (bind _modechoosen (`MPIAPlayerController.ModeChoosen` _asbp_mpiaplayer_controller))
    (if (== _modechoosen 0)
      (`self.OneWay` _outactors)
      (elif (== _modechoosen 1)
        _
        (elif (== _modechoosen 2)
          (`self.Circuit` _outactors))))))

(fn `UserConstructionScript`)